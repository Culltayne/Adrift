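; BP_Rambling is a dialogue audio Blueprint that plays the MSS_Rambling sound, likely a MetaSound, attached to the third-person character.
; On BeginPlay it casts the owner of the SpotLight's capsule to BP_ThirdPersonCharacter and spawns the sound on that character's parent component.
; On Destroyed it sends a "None" trigger parameter to the sound.
; Leftover random-delay and variation logic is disconnected and never runs.
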(event `self.ReceiveDestroyed`
  (`AudioParameterControllerInterface.SetTriggerParameter` (stale `self.ReceiveBeginPlay` _returnvalue) "None"))

(event `self.ReceiveBeginPlay`
  (bind _asbp_third_person_character (cast `/Game/ThirdPerson/Blueprints/BP_ThirdPersonCharacter` (`ActorComponent.GetOwner` (`Character.CapsuleComponent` (`self.SpotLight`)))))
  (bind _returnvalue (`GameplayStatics.SpawnSoundAttached` "/Game/Audio/Dialogue/MSS_Rambling.MSS_Rambling" (`self.GetParentComponent` _asbp_third_person_character) "None" (0.0 0.0 0.0) (struct) "KeepRelativeOffset" false 1.0 1.0 0.0 null null)))

(fn `UserConstructionScript`)