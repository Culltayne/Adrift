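; BP_ProgPickup_A is a collectible pickup that adds a random amount of score when the player character touches it.
; A Timeline started on BeginPlay drives the Sphere's relative Z to animate its height.
; Box overlap with BP_ThirdPersonCharacter increases Score on the ProgPrac actor found by class lookup.
; It then destroys the pickup, plays a 2D coin sound and prints the new score on screen.
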(event `self.ReceiveBeginPlay`
  (bind (_direction _verticalheight) (`Timeline|Timeline`)
    (:`Update`
      (`SceneComponent.K2_SetRelativeLocation` (`self.Sphere`) (`KismetMathLibrary.MakeVector` 0.0 0.0 (* _verticalheight 100.0)) false false))))

(event `self.Box.OnComponentBeginOverlap`
  (params (OverlappedComponent :type "PrimitiveComponent Object Reference") (OtherActor :type "Actor Object Reference") (OtherComp :type "PrimitiveComponent Object Reference") (OtherBodyIndex :type Integer) (bFromSweep :type Boolean) (SweepResult :type "HitResult Structure (by ref)"))
  (cast `/Game/ThirdPerson/Blueprints/BP_ThirdPersonCharacter` OtherActor)
  (bind _returnvalue (`GameplayStatics.GetActorOfClass` "/Game/ProgPrac/ProgPrac.ProgPrac_C"))
  (bind _output_get (set `/Game/ProgPrac/ProgPrac.Score` (+ (`/Game/ProgPrac/ProgPrac.Score` _returnvalue) (`KismetMathLibrary.RandomIntegerInRange` 5 10)) _returnvalue))
  (`self.K2_DestroyActor`)
  (`GameplayStatics.PlaySound2D` "/Game/ProgPrac/collectcoin-6075.collectcoin-6075" 1.0 1.0 0.0 null null)
  (`KismetSystemLibrary.PrintString` (`KismetStringLibrary.Conv_IntToString` _output_get) true true (struct :`R` 1.0 :`G` 0.032916 :`A` 1.0) 5.0))

(fn `UserConstructionScript`)