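; BP_Console is an interactable console actor that plays the ADRIFT_D12 sound when used.
; Its Box overlap shows a W_InteractItem prompt and removes it on exit, without checking which actor overlaps.
; Interactwith plays the sound at world origin through a DoOnce that resets after 15 seconds.
; Unconnected leftover chains hold a HUD widget reset and a looping randomized screen sound.
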(event `/Game/Blueprints/BPI_Interface.InteractWith`
  (`/Engine/EditorBlueprintResources/StandardMacros.DoOnce` false :!label _label
    (:`Completed`
      (`GameplayStatics.PlaySoundAtLocation` "/Game/Audio/Jack/ADRIFT_D12.ADRIFT_D12" (0.0 0.0 0.0) (struct) 1.0 1.0 0.0 null null null null)
      (`KismetSystemLibrary.Delay` 15.0)
      (goto _label :!via `Reset`))))

(event `self.Box.OnComponentBeginOverlap`
  (params (OverlappedComponent :type "PrimitiveComponent Object Reference") (OtherActor :type "Actor Object Reference") (OtherComp :type "PrimitiveComponent Object Reference") (OtherBodyIndex :type Integer) (bFromSweep :type Boolean) (SweepResult :type "HitResult Structure (by ref)"))
  (bind _returnvalue (`|CreateWidget` "/Game/WidgetsUI/W_InteractItem.W_InteractItem_C"))
  (`UserWidget.AddToViewport` _returnvalue 0))

(event `self.Box.OnComponentEndOverlap`
  (params (OverlappedComponent :type "PrimitiveComponent Object Reference") (OtherActor :type "Actor Object Reference") (OtherComp :type "PrimitiveComponent Object Reference") (OtherBodyIndex :type Integer))
  (`Widget.RemoveFromParent` (stale `self.Box.OnComponentBeginOverlap` _returnvalue)))

(event `self.ReceiveBeginPlay`)

(fn `UserConstructionScript`)